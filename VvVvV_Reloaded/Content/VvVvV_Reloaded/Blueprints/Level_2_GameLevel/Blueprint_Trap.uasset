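; Trap actor that roots an enemy Thief player character in place when they step on it in the game level.
; It arms two seconds after spawning and ignores its OwnerCharacter.
; On overlap it plays a sound, reveals its cylinder mesh and zeroes the victim's MaxWalkSpeed for TrapDuration, then restores the saved speed and destroys itself.
; CanTrigger is never cleared on triggering, and the TriggerTrap event is empty.
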(event `self.ReceiveBeginPlay`
  (`KismetSystemLibrary.Delay` 2.0)
  (set `self.CanTrigger` true))

(event `self.ReceiveActorBeginOverlap`
  (params (OtherActor :type "Actor Object Reference"))
  (if (`self.CanTrigger`)
    (bind _asplayer_character_game_level_thief (cast `/Game/VvVvV_Reloaded/Blueprints/Level_2_GameLevel/PlayerCharacter_GameLevel_Thief` OtherActor))
    (if (!= _asplayer_character_game_level_thief (`self.OwnerCharacter`))
      (set `self.OtherCharacterMovement` (`Character.CharacterMovement` _asplayer_character_game_level_thief))
      (`GameplayStatics.PlaySoundAtLocation` "/Game/VvVvV_Reloaded/Audio/TrapTriggeringSound.TrapTriggeringSound" (`SceneComponent.K2_GetComponentLocation` (`self.Cylinder`)))
      (`SceneComponent.SetVisibility` (`self.Cylinder`) true true)
      (set `self.MaxWalkSpeed` (`CharacterMovementComponent.MaxWalkSpeed` (`self.OtherCharacterMovement`)))
      (set `CharacterMovementComponent.MaxWalkSpeed` 0.0 (`self.OtherCharacterMovement`))
      (`KismetSystemLibrary.Delay` (`self.TrapDuration`))
      (set `CharacterMovementComponent.MaxWalkSpeed` (`self.MaxWalkSpeed`) (`self.OtherCharacterMovement`))
      (`self.K2_DestroyActor`))))

(event `TriggerTrap`)

(fn `UserConstructionScript`)