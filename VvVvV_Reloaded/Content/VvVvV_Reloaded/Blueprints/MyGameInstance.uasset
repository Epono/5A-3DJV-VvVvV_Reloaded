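; Game instance Blueprint that manages LAN multiplayer sessions and level travel through custom events.
; Hosting creates a four-connection session and opens MainGameMap as a listen server, while joining searches for one session and joins the first result.
; Other events run a servertravel console command for a given level or destroy the session.
; Session creation and search failures only print on-screen errors.
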(event `Instance_HostLobby`
  (params (Host :type "PlayerController Object Reference"))
  (`CreateSessionCallbackProxy.CreateSession` Host 4 true
    (:`OnSuccess`
      (`GameplayStatics.OpenLevel` "MainGameMap" true "listen"))
    (:`OnFailure`
      (`KismetSystemLibrary.PrintString` "ERREUR CREATION SESSION" true true (struct :`R` 1.0 :`B` 0.109378 :`A` 1.0)))))

(event `Instance_JoinLobby`
  (params (Joining :type "PlayerController Object Reference"))
  (bind _results (`FindSessionsCallbackProxy.FindSessions` Joining 1 true)
    (:`OnSuccess`
      (`JoinSessionCallbackProxy.JoinSession` Joining (`KismetArrayLibrary.Array_Get` _results)))
    (:`OnFailure`
      (`KismetSystemLibrary.PrintString` "SESSION SEARCH FAILED" true true (struct :`R` 1.0 :`B` 0.109378 :`A` 1.0)))))

(event `Instance_TravelToLevel`
  (params (LevelToLoad :type String))
  (`KismetSystemLibrary.ExecuteConsoleCommand` (`KismetStringLibrary.Concat_StrStr` "servertravel " LevelToLoad) (`GameplayStatics.GetPlayerController` 0)))

(event `Instance_DestroySession`
  (`DestroySessionCallbackProxy.DestroySession` null))