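; Player controller for the lobby level that owns the lobby HUD and starts the game.
; On BeginPlay it creates and shows the HUD_Lobby widget, removing it on EndPlay.
; A play event hands the controller to GameInstance_VvVvV to launch play.
; Other events forward the loading screen and pre-launch countdown updates to the HUD.
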(event `self.ReceiveBeginPlay`
  ;[1 1 1] HUD initialization
  (bind _returnvalue (`|CreateWidget` "/Game/VvVvV_Reloaded/HUD/HUD_Lobby.HUD_Lobby_C" (`GameplayStatics.GetPlayerController` 0)))
  (bind _output_get (set `self.Menu` _returnvalue))
  (`UserWidget.AddToViewport` _output_get 0)
  (`Widget.SetVisibility` _returnvalue "Visible"))

(event `self.ReceiveEndPlay`
  (params (EndPlayReason :type "EEndPlayReason Enum" :default "Destroyed"))
  ;[1 1 1] Destroying HUD
  (`Widget.RemoveFromParent` (`self.Menu`)))

(event `PlayerServer_Play`
  ;[1 1 1] PLAY !
  (bind _asgame_instance_vv_vv_v (cast `/Game/VvVvV_Reloaded/Blueprints/GameInstance_VvVvV` (`GameplayStatics.GetGameInstance`)))
  (`/Game/VvVvV_Reloaded/Blueprints/GameInstance_VvVvV.Instance_Play` _asgame_instance_vv_vv_v self))

(event `DisplayLoadingScreen`
  ;[1 1 1] Displays loading screen and loading text
  (`/Game/VvVvV_Reloaded/HUD/HUD_Lobby.DisplayLoadingScreen` (`self.Menu`)))

(event `ChangeTimeBeforeLaunch`
  (params (TimeBeforeLaunch :type Integer))
  ;[1 1 1] Displays time before launch
  (`/Game/VvVvV_Reloaded/HUD/HUD_Lobby.ChangeTimeBeforeLaunch` (`self.Menu`) TimeBeforeLaunch))

(fn `UserConstructionScript`)