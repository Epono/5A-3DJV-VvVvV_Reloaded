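; Lobby player controller that gives the player a travel menu for hosting, joining and changing levels.
; After a short delay on BeginPlay, the authority calls the client-named event that creates the hidden HUD_TravelMenu widget.
; The OpenMenu input toggles the menu's visibility and switches input mode between game-only and game-and-UI.
; Server-named events forward host, join and level-travel requests to MyGameInstance, and EndPlay removes the widget.
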(event `self.ReceiveBeginPlay`
  ;[1 1 1] HUD initialization
  (`KismetSystemLibrary.Delay` 2.0)
  (`/Engine/EditorBlueprintResources/ActorMacros.Switch Has Authority`
    (:`Authority`
      (`self.PlayerClient_CreateHUD`))))

(event `PlayerClient_CreateHUD`
  ;[1 1 1] HUD initialization
  (bind _returnvalue (`|CreateWidget` "/Game/VvVvV_Reloaded/HUD/HUD_TravelMenu.HUD_TravelMenu_C" (`GameplayStatics.GetPlayerController` 0)))
  (bind _output_get (set `self.Player_TravelMenu` _returnvalue))
  (`UserWidget.AddToViewport` _output_get 0)
  (`Widget.SetVisibility` _returnvalue "Hidden"))

(event `InputAction|OpenMenu`
  (params (Key :type "Key Structure" :default "AnyKey"))
  (bind _player_travelmenu (`self.Player_TravelMenu`))
  ;[1 1 1] Open Menu
  (:`Pressed`
    (if (`|EnumEquality` (`Widget.GetVisibility` _player_travelmenu) "Visible")
      (`Widget.SetVisibility` _player_travelmenu "Hidden")
      (`WidgetBlueprintLibrary.SetInputMode_GameOnly` self)
      (else
        (`Widget.SetVisibility` _player_travelmenu "Visible")
        (`WidgetBlueprintLibrary.SetInputMode_GameAndUIEx` self)))))

(event `PlayerServer_HostLobby`
  (bind _asmy_game_instance (cast `/Game/VvVvV_Reloaded/Blueprints/MyGameInstance` (`GameplayStatics.GetGameInstance`)))
  (`/Game/VvVvV_Reloaded/Blueprints/MyGameInstance.Instance_HostLobby` _asmy_game_instance self))

(event `self.ReceiveEndPlay`
  (params (EndPlayReason :type "EEndPlayReason Enum" :default "Destroyed"))
  (`Widget.RemoveFromParent` (`self.Player_TravelMenu`)))

(event `PlayerServer_JoinLobby`
  (bind _asmy_game_instance (cast `/Game/VvVvV_Reloaded/Blueprints/MyGameInstance` (`GameplayStatics.GetGameInstance`)))
  (`/Game/VvVvV_Reloaded/Blueprints/MyGameInstance.Instance_JoinLobby` _asmy_game_instance self))

(event `PlayerServer_TravelToNewLevel`
  (params (LevelToLoad :type String))
  (bind _asmy_game_instance (cast `/Game/VvVvV_Reloaded/Blueprints/MyGameInstance` (`GameplayStatics.GetGameInstance`)))
  (`/Game/VvVvV_Reloaded/Blueprints/MyGameInstance.Instance_TravelToLevel` _asmy_game_instance LevelToLoad))

(fn `UserConstructionScript`)