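; Player character for the lobby level that moves relative to control yaw, faces the cursor and fires projectiles.
; BeginPlay attaches a baguette weapon to a mesh socket.
; Tick caches the lobby controller, then yaws toward the cursor hit, applying it locally and through ServerSetActorRotation.
; Left click plays a shot sound and calls NetworkSpawProjectile, which spawns the projectile and explosion particles; ChangePlayerMaterial swaps the billboard sprite by index.
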(event `self.ReceiveBeginPlay`
  (bind (_returnvalue_location _returnvalue_rotation) (`KismetMathLibrary.BreakTransform` (`self.GetTransform`)))
  ;[1 1 1] Instanciation de l'arme
  (bind _returnvalue (`|SpawnActorFromClass` "/Game/VvVvV_Reloaded/Weapons/FPWeapon/Mesh/BaguetteBlueprint.BaguetteBlueprint_C" (`KismetMathLibrary.MakeTransform` _returnvalue_location _returnvalue_rotation (2.0 2.0 1.0)) "Undefined" "OverrideRootScale"))
  (`self.K2_AttachRootComponentTo` _returnvalue (`self.Mesh`) "BaguetteSocket" "SnapToTarget" true)
  (set `self.GunReference` null))

(event `InputAxis|MoveRight`
  (params (AxisValue :type "Float (single-precision)"))
  (bind (_returnvalue_roll _returnvalue_pitch _returnvalue_yaw) (`KismetMathLibrary.BreakRotator` (`self.GetControlRotation`)))
  ;[1 1 1] Lateral Movement
  (`self.AddMovementInput` (`KismetMathLibrary.GetRightVector` (`KismetMathLibrary.MakeRotator` 0.0 0.0 _returnvalue_yaw)) AxisValue))

(event `InputAxis|MoveForward`
  (params (AxisValue :type "Float (single-precision)"))
  (bind (_returnvalue_roll _returnvalue_pitch _returnvalue_yaw) (`KismetMathLibrary.BreakRotator` (`self.GetControlRotation`)))
  ;[1 1 1] Vertical Movement
  (`self.AddMovementInput` (`KismetMathLibrary.GetForwardVector` (`KismetMathLibrary.MakeRotator` 0.0 0.0 _returnvalue_yaw)) AxisValue))

(event `self.ReceiveTick`
  (params (DeltaSeconds :type "Float (single-precision)"))
  (bind (_returnvalue_roll _returnvalue_pitch _returnvalue_yaw) (`KismetMathLibrary.BreakRotator` (`KismetMathLibrary.FindLookAtRotation` (`self.K2_GetActorLocation` self) (`.Location` (`GameplayStatics.BreakHitResult` (`PlayerController.GetHitResultUnderCursorByChannel` (`self.ControllerReference`) "TraceTypeQuery1" true))))))
  (bind _returnvalue (`KismetMathLibrary.MakeRotator` 0.0 0.0 _returnvalue_yaw))
  ;[1 1 1] Tick (rotation)
  (if (`KismetSystemLibrary.IsValid` (`self.ControllerReference`))
    (if (`self.IsLocallyControlled`)
      (`self.SetActorRotation` _returnvalue :!label _label)
      (`self.ServerSetActorRotation` _returnvalue))
    (else
      (bind _asplayer_controller_lobby (cast `/Game/VvVvV_Reloaded/Blueprints/Level_1_Lobby/PlayerController_Lobby` (`self.GetController`)))
      (set `self.ControllerReference` _asplayer_controller_lobby)
      (goto _label))))

(event `ServerSetActorRotation`
  (params (Rotation :type "Rotator Structure"))
  ;[1 1 1] Tick (rotation)
  (`self.SetActorRotation` Rotation))

(event `Key|LeftMouseButton`
  (params (Key :type "Key Structure" :default "AnyKey"))
  (bind (_returnvalue_roll _returnvalue_pitch _returnvalue_yaw) (`KismetMathLibrary.BreakRotator` (`KismetMathLibrary.FindLookAtRotation` (`self.K2_GetActorLocation` self) (`.Location` (`GameplayStatics.BreakHitResult` (`PlayerController.GetHitResultUnderCursorByChannel` (`self.ControllerReference`) "TraceTypeQuery1" true))))))
  (bind _returnvalue (`KismetMathLibrary.MakeRotator` 0.0 0.0 _returnvalue_yaw))
  (bind _returnvalue_2 (+ (* (`KismetMathLibrary.GetForwardVector` _returnvalue) 150.0) (`self.K2_GetActorLocation` self)))
  ;[1 1 1] Launch cube !
  (:`Pressed`
    (`self.NetworkSpawProjectile` (`KismetMathLibrary.MakeTransform` _returnvalue_2 _returnvalue))
    (`GameplayStatics.PlaySoundAtLocation` "/Game/VvVvV_Reloaded/Audio/ShotSound.ShotSound" _returnvalue_2 (struct) 0.05)))

(event `NetworkSpawProjectile`
  (params (Transform :type "Transform Structure"))
  ;[1 1 1] Launch cube !
  (`|SpawnActorFromClass` "/Game/VvVvV_Reloaded/Blueprints/Level_2_GameLevel/Blueprint_Projectile.Blueprint_Projectile_C" Transform "AdjustIfPossibleButAlwaysSpawn" "OverrideRootScale")
  (`self.PlaySoundAndSpawnParticlesShot`))

(event `PlaySoundAndSpawnParticlesShot`
  (bind (_returnvalue_roll _returnvalue_pitch _returnvalue_yaw) (`KismetMathLibrary.BreakRotator` (`KismetMathLibrary.FindLookAtRotation` (`self.K2_GetActorLocation` self) (`.Location` (`GameplayStatics.BreakHitResult` (`PlayerController.GetHitResultUnderCursorByChannel` (`self.ControllerReference`) "TraceTypeQuery1" true))))))
  ;[1 1 1] Launch cube !
  (`GameplayStatics.SpawnEmitterAtLocation` "/Game/StarterContent/Particles/P_Explosion.P_Explosion" (+ (`SceneComponent.GetSocketLocation` (`self.Mesh`) "BaguetteSocket") (* (`KismetMathLibrary.GetForwardVector` (`KismetMathLibrary.MakeRotator` 0.0 0.0 _returnvalue_yaw)) 75.0))))

(event `ChangePlayerMaterial`
  (params (Index :type Integer))
  (bind _billboard (`self.Billboard`))
  (switch `int` Index
    (:`0`
      (`BillboardComponent.SetSprite` _billboard "/Game/VvVvV_Reloaded/Images/1.1"))
    (:`1`
      (`BillboardComponent.SetSprite` _billboard "/Game/VvVvV_Reloaded/Images/2.2"))
    (:`2`
      (`BillboardComponent.SetSprite` _billboard "/Game/VvVvV_Reloaded/Images/3.3"))
    (:`3`
      (`BillboardComponent.SetSprite` _billboard "/Game/VvVvV_Reloaded/Images/4.4"))))

(fn `UserConstructionScript`
  (cast `/Game/VvVvV_Reloaded/Blueprints/Level_2_GameLevel/PlayerController_GameLevel_Thief` (`self.GetController`))
  (set `self.ControllerReference` null))