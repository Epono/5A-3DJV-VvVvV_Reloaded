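; Game Instance for VvVvV that manages LAN multiplayer sessions through custom events for hosting, joining, level travel and teardown.
; Hosting creates a four-slot session, then opens the lobby level as a listen server.
; Joining searches for one LAN session and joins it, with host and search failures printed on screen.
; Game level changes run a servertravel console command, and a separate event destroys the session.
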(event `Instance_Host`
  (params (Host :type "PlayerController Object Reference"))
  ;[1 1 1] Hosting
  (`CreateSessionCallbackProxy.CreateSession` Host 4 true
    (:`OnSuccess`
      (`GameplayStatics.OpenLevel` "Level_1_Lobby" true "listen"))
    (:`OnFailure`
      (`KismetSystemLibrary.PrintString` "ERREUR CREATION SESSION" true true (struct :`R` 1.0 :`B` 0.109378 :`A` 1.0)))))

(event `Instance_Join`
  (params (Joining :type "PlayerController Object Reference"))
  ;[1 1 1] Joining
  (bind _results (`FindSessionsCallbackProxy.FindSessions` Joining 1 true)
    (:`OnSuccess`
      (if (!= (`KismetArrayLibrary.Array_Length` _results) 0)
        (`JoinSessionCallbackProxy.JoinSession` Joining (`KismetArrayLibrary.Array_Get` _results))))
    (:`OnFailure`
      (`KismetSystemLibrary.PrintString` "SESSION SEARCH FAILED" true true (struct :`R` 1.0 :`B` 0.109378 :`A` 1.0)))))

(event `Instance_TravelToGameLevel`
  (params (LevelToLoad :type String))
  ;[1 1 1] Travelling to GameLevel
  (`KismetSystemLibrary.ExecuteConsoleCommand` (`KismetStringLibrary.Concat_StrStr` "servertravel " LevelToLoad) (`GameplayStatics.GetPlayerController` 0)))

(event `Instance_DestroySession`
  ;[1 1 1] Destroying session
  (`DestroySessionCallbackProxy.DestroySession` null))