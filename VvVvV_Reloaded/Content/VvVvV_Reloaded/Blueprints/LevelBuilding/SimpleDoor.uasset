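; SimpleDoor is a level-building door that opens when something overlaps its trigger and closes when the overlap ends.
; The DoorMove timeline drives the Door component's relative location, playing forward on begin overlap and reversing on end overlap.
; Pressing E, with no overlap check, moves the whole actor to 200 units from the trigger along world Y or X, depending on whether trigger rotation is zero.
; A Thief_PlayerCharacter cast is left unconnected.
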(event `self.ReceiveActorBeginOverlap`
  (params (OtherActor :type "Actor Object Reference")))

(event `self.ReceiveBeginPlay`)

(event `self.ReceiveTick`
  (params (DeltaSeconds :type "Float (single-precision)")))

(event `self.DoorTrigger.OnComponentBeginOverlap`
  (params (OtherActor :type "Actor Object Reference") (OtherComp :type "PrimitiveComponent Object Reference") (OtherBodyIndex :type Integer) (bFromSweep :type Boolean) (SweepResult :type "HitResult Structure (by ref)"))
  (bind (_direction _door_movement) (`Timeline|DoorMove` :!label _label)
    (:`Update`
      (`SceneComponent.K2_SetRelativeLocation` (`self.Door`) _door_movement false false))))

(event `self.DoorTrigger.OnComponentEndOverlap`
  (params (OtherActor :type "Actor Object Reference") (OtherComp :type "PrimitiveComponent Object Reference") (OtherBodyIndex :type Integer))
  (goto _label :!via `Reverse`))

(event `Key|E`
  (params (Key :type "Key Structure" :default "AnyKey"))
  (bind _location (.location (`SceneComponent.K2_GetComponentToWorld` (`self.DoorTrigger`))))
  (:`Pressed`
    (if true
      (if (== (.rotation (`SceneComponent.K2_GetComponentToWorld` (`self.DoorTrigger`))) (struct))
        (`self.K2_SetActorLocation` (+ _location (0.0 200.0 0.0)))
        (else
          (`self.K2_SetActorLocation` (+ _location (200.0 0.0 0.0))))))))

(fn `UserConstructionScript`)