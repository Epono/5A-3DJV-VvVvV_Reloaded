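; Player controller for the Thief, handling trap placement and mouse-driven aiming.
; SetTrap spawns a Trap_BP at its own transform with a fixed height, sets itself as owner, plays a sound, then blocks placement for TrapDelay; early presses print a TODO message.
; Tick yaws player character 0 toward the point under the cursor.
; An unused click-to-move function remains, reusing TrapDelay as its minimum distance.
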(event `InputAction|SetTrap`
  (params (Key :type "Key Structure" :default "AnyKey"))
  (bind _returnvalue (`SceneComponent.K2_GetComponentToWorld` (`self.TransformComponent`)))
  (bind _returnvalue_2 (`KismetMathLibrary.MakeTransform` (`KismetMathLibrary.MakeVector` (.x (.location _returnvalue)) (.y (.location _returnvalue)) 170.0) (.rotation _returnvalue) (.scale _returnvalue)))
  ;[1 1 1] Set trap
  (:`Pressed`
    (if (`self.CanSetTrap`)
      (bind _returnvalue_3 (`|SpawnActorFromClass` "/Game/VvVvV_Reloaded/Blueprints/Trap_BP.Trap_BP_C" _returnvalue_2 "Undefined" "OverrideRootScale"))
      (set `/Game/VvVvV_Reloaded/Blueprints/Trap_BP.OwnerCharacter` self _returnvalue_3)
      (`GameplayStatics.PlaySoundAtLocation` "/Game/VvVvV_Reloaded/Audio/TrapSettingSound.TrapSettingSound" (.location _returnvalue_2))
      (set `self.CanSetTrap` false)
      (`KismetSystemLibrary.Delay` (`self.TrapDelay`))
      (set `self.CanSetTrap` true)
      (else
        (`KismetSystemLibrary.PrintString` "TODO: message d'erreur qu'on peut pas encore reposer de piège")))))

(event `self.ReceiveTick`
  (params (DeltaSeconds :type "Float (single-precision)"))
  (bind _returnvalue (`GameplayStatics.GetPlayerCharacter` 0))
  (bind (_returnvalue_roll _returnvalue_pitch _returnvalue_yaw) (`KismetMathLibrary.BreakRotator` (`KismetMathLibrary.FindLookAtRotation` (`self.K2_GetActorLocation` _returnvalue) (`.Location` (`GameplayStatics.BreakHitResult` (`self.GetHitResultUnderCursorByChannel` "TraceTypeQuery1"))))))
  ;[1 1 1] Tick (rotation)
  (`self.SetActorRotation` _returnvalue (`KismetMathLibrary.MakeRotator` 0.0 0.0 _returnvalue_yaw)))

(fn `MoveToHitLocation`
  (params (Hit :type "HitResult Structure"))
  (bind (_bblockinghit _binitialoverlap _time _location) (`GameplayStatics.BreakHitResult` Hit))
  (if (>= (`KismetMathLibrary.VSize` (- (`self.K2_GetActorLocation` (`self.K2_GetPawn`)) _location)) (`self.TrapDelay`))
    (`NavigationSystem.SimpleMoveToLocation` self _location) ; Send the destination point to the character
  ))

(fn `UserConstructionScript`)