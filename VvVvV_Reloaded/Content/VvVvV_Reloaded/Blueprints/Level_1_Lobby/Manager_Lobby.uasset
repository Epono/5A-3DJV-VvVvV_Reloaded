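; Lobby manager that plays background music and lets the server launch the match with the Enter key.
; A one-shot countdown prints to screen and pushes the remaining seconds to up to four lobby player controllers.
; At zero, the authority has each controller display a loading screen, waits briefly so clients show it, then the game instance travels to the game level.
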(event `Key|Enter`
  (params (Key :type "Key Structure" :default "AnyKey"))
  ;[1 1 1] Server starts game
  (:`Pressed`
    (if (`KismetSystemLibrary.IsServer`)
      (`/Engine/EditorBlueprintResources/StandardMacros.DoOnce` false
        (:`Completed`
          (`KismetSystemLibrary.PrintString` "Game will start in 3 ..." true true (struct :`G` 0.66 :`B` 1.0 :`A` 1.0) 5.0)
          (`self.ChangeTimeBeforeLaunch` 3)
          (`KismetSystemLibrary.Delay` 1.0)
          (`KismetSystemLibrary.PrintString` "2 ..." true true (struct :`G` 0.66 :`B` 1.0 :`A` 1.0) 5.0)
          (`self.ChangeTimeBeforeLaunch` 2)
          (`KismetSystemLibrary.Delay` 1.0)
          (`KismetSystemLibrary.PrintString` "1 ..." true true (struct :`G` 0.66 :`B` 1.0 :`A` 1.0) 5.0)
          (`self.ChangeTimeBeforeLaunch` 1)
          (`KismetSystemLibrary.Delay` 1.0)
          (`self.ChangeTimeBeforeLaunch` 0)
          (bind _asgame_instance_vv_vv_v (cast `/Game/VvVvV_Reloaded/Blueprints/GameInstance_VvVvV` (`GameplayStatics.GetGameInstance`)))
          (`/Engine/EditorBlueprintResources/ActorMacros.Switch Has Authority`
            (:`Authority`
              (`self.GameStarts`)
              ;;[1 1 1] Sinon y'a un client pour lequel ça affihe pas l'écran de chargeent
              (`KismetSystemLibrary.Delay` 0.5)
              (`/Game/VvVvV_Reloaded/Blueprints/GameInstance_VvVvV.Instance_TravelToGameLevel` _asgame_instance_vv_vv_v "Level_2_GameLevel"))))))))

(event `GameStarts`
  ;[1 1 1] Server starts game
  (for _index (range 4)
    (bind _asplayer_controller_lobby (cast `/Game/VvVvV_Reloaded/Blueprints/Level_1_Lobby/PlayerController_Lobby` (`GameplayStatics.GetPlayerController` _index)))
    (`/Game/VvVvV_Reloaded/Blueprints/Level_1_Lobby/PlayerController_Lobby.DisplayLoadingScreen` _asplayer_controller_lobby)))

(event `self.ReceiveBeginPlay`
  ;[1 1 1] Background music
  (`GameplayStatics.PlaySound2D` "/Game/VvVvV_Reloaded/Audio/Lobby_BackgroundMusic.Lobby_BackgroundMusic" 0.05))

(fn `ChangeTimeBeforeLaunch`
  (params (TimeBeforeLaunch :type Integer))
  (for _index (range 4)
    (bind _asplayer_controller_lobby (cast `/Game/VvVvV_Reloaded/Blueprints/Level_1_Lobby/PlayerController_Lobby` (`GameplayStatics.GetPlayerController` _index)))
    (`/Game/VvVvV_Reloaded/Blueprints/Level_1_Lobby/PlayerController_Lobby.ChangeTimeBeforeLaunch` _asplayer_controller_lobby TimeBeforeLaunch)))

(fn `UserConstructionScript`)