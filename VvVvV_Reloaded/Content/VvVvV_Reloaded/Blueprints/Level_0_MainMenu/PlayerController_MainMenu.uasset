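; Main menu player controller that shows the menu HUD and starts multiplayer sessions.
; On BeginPlay it creates the HUD_MainMenu widget and adds it to the viewport, then removes it on EndPlay.
; Its host and join events cast to GameInstance_VvVvV and pass the controller to that instance's InstanceHost or InstanceJoin.
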(event `self.ReceiveBeginPlay`
  ;[1 1 1] HUD initialization
  (bind _returnvalue (`|CreateWidget` "/Game/VvVvV_Reloaded/HUD/HUD_MainMenu.HUD_MainMenu_C" (`GameplayStatics.GetPlayerController` 0)))
  (bind _output_get (set `self.Menu` _returnvalue))
  (`UserWidget.AddToViewport` _output_get 0)
  (`Widget.SetVisibility` _returnvalue "Visible"))

(event `PlayerServer_Host`
  ;[1 1 1] Hosting
  (bind _asgame_instance_vv_vv_v (cast `/Game/VvVvV_Reloaded/Blueprints/GameInstance_VvVvV` (`GameplayStatics.GetGameInstance`)))
  (`/Game/VvVvV_Reloaded/Blueprints/GameInstance_VvVvV.Instance_Host` _asgame_instance_vv_vv_v self))

(event `self.ReceiveEndPlay`
  (params (EndPlayReason :type "EEndPlayReason Enum" :default "Destroyed"))
  ;[1 1 1] Destroying HUD
  (`Widget.RemoveFromParent` (`self.Menu`)))

(event `PlayerServer_Join`
  ;[1 1 1] Joining
  (bind _asgame_instance_vv_vv_v (cast `/Game/VvVvV_Reloaded/Blueprints/GameInstance_VvVvV` (`GameplayStatics.GetGameInstance`)))
  (`/Game/VvVvV_Reloaded/Blueprints/GameInstance_VvVvV.Instance_Join` _asgame_instance_vv_vv_v self))

(fn `UserConstructionScript`)