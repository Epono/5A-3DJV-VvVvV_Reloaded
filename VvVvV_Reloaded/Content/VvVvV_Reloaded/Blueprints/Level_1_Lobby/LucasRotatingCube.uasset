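; Decorative lobby actor that tumbles and pulses a cube while sweeping its spring arm around it.
; Tick accumulates a scaled time value that drives the cube's roll and pitch together.
; The same value feeds a squared cosine for a bouncing uniform scale and, at half rate, the spring arm's yaw.
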(event `self.ReceiveBeginPlay`)

(event `self.ReceiveActorBeginOverlap`
  (params (OtherActor :type "Actor Object Reference")))

(event `self.ReceiveTick`
  (params (DeltaSeconds :type "Float (single-precision)"))
  (bind _timeelapsed (`self.TimeElapsed`))
  (bind _cube (`self.Cube`))
  ;[1 1 1] Rotation
  (bind _output_get (set `self.TimeElapsed` (+ (* DeltaSeconds 50.0) _timeelapsed)))
  (`SceneComponent.K2_SetRelativeRotation` _cube (`KismetMathLibrary.MakeRotator` _output_get _output_get) false false)
  ;[1 1 1] Bounce
  (`SceneComponent.SetRelativeScale3D` _cube (`KismetMathLibrary.Conv_DoubleToVector` (* (+ (* (`KismetMathLibrary.Square` (`KismetMathLibrary.DegCos` _timeelapsed)) 2.0) 1.0) 2.0)))
  (`SceneComponent.K2_SetRelativeRotation` (`self.SpringArm`) (`KismetMathLibrary.MakeRotator` 0.0 0.0 (/ _timeelapsed 2.0)) false false))

(fn `UserConstructionScript`)