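; Player character for the Thief in the game level, with camera-relative movement, stepped spring-arm zoom and a coin score.
; Each tick it yaws toward the point under the cursor via the cached Thief controller, passing the rotation through server and client events.
; Left click fires a projectile toward the cursor through a network spawn event, and SetTrap drops a trap at a fixed height, both gated by cooldown flags.
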(event `InputAction|ZoomIn`
  (params (Key :type "Key Structure" :default "AnyKey"))
  (bind _springarm1 (`self.SpringArm1`))
  ;[1 1 1] Zoom
  (:`Pressed`
    (set `SpringArmComponent.TargetArmLength` (+ -100.0 (`SpringArmComponent.TargetArmLength` _springarm1)) _springarm1)))

(event `InputAction|ZoomOut`
  (params (Key :type "Key Structure" :default "AnyKey"))
  (bind _springarm1 (`self.SpringArm1`))
  ;[1 1 1] Zoom
  (:`Pressed`
    (set `SpringArmComponent.TargetArmLength` (+ 100.0 (`SpringArmComponent.TargetArmLength` _springarm1)) _springarm1)))

(event `InputAxis|MoveRight`
  (params (AxisValue :type "Float (single-precision)"))
  (bind (_returnvalue_roll _returnvalue_pitch _returnvalue_yaw) (`KismetMathLibrary.BreakRotator` (`self.GetControlRotation`)))
  ;[1 1 1] Lateral Movement
  (`self.AddMovementInput` (`KismetMathLibrary.GetRightVector` (`KismetMathLibrary.MakeRotator` 0.0 0.0 _returnvalue_yaw)) AxisValue))

(event `InputAxis|MoveForward`
  (params (AxisValue :type "Float (single-precision)"))
  (bind (_returnvalue_roll _returnvalue_pitch _returnvalue_yaw) (`KismetMathLibrary.BreakRotator` (`self.GetControlRotation`)))
  ;[1 1 1] Vertical Movement
  (`self.AddMovementInput` (`KismetMathLibrary.GetForwardVector` (`KismetMathLibrary.MakeRotator` 0.0 0.0 _returnvalue_yaw)) AxisValue))

(event `CoinPickedUp`
  ;[1 1 1] Coin picked up
  (set `self.Score` (+ 1 (`self.Score`))))

(event `InputAction|SetTrap`
  (params (Key :type "Key Structure" :default "AnyKey"))
  (bind (_returnvalue_x _returnvalue_y) (`KismetMathLibrary.BreakVector` (`SceneComponent.K2_GetComponentLocation` (`self.CapsuleComponent`))))
  (bind _returnvalue (`KismetMathLibrary.MakeVector` _returnvalue_x _returnvalue_y 170.0))
  ;[1 1 1] Set trap
  (:`Pressed`
    (if (`self.CanSetTrap`)
      (`|SpawnActorFromClass` "/Game/VvVvV_Reloaded/Blueprints/Level_2_GameLevel/Blueprint_Trap.Blueprint_Trap_C" (`KismetMathLibrary.Conv_VectorToTransform` _returnvalue) "Undefined" "OverrideRootScale")
      (`GameplayStatics.PlaySoundAtLocation` "/Game/VvVvV_Reloaded/Audio/TrapSettingSound.TrapSettingSound" _returnvalue)
      (set `self.CanSetTrap` false)
      (`KismetSystemLibrary.Delay` (`self.TrapDelay`))
      (set `self.CanSetTrap` true)
      (else
        (`KismetSystemLibrary.PrintString` "TODO: message d'erreur qu'on peut pas encore reposer de piège")))))

(event `self.ReceiveTick`
  (params (DeltaSeconds :type "Float (single-precision)"))
  (bind (_returnvalue_roll _returnvalue_pitch _returnvalue_yaw) (`KismetMathLibrary.BreakRotator` (`KismetMathLibrary.FindLookAtRotation` (`self.K2_GetActorLocation` self) (`.Location` (`GameplayStatics.BreakHitResult` (`PlayerController.GetHitResultUnderCursorByChannel` (`self.ControllerReference`) "TraceTypeQuery1" true))))))
  (bind _returnvalue (`KismetMathLibrary.MakeRotator` 0.0 0.0 _returnvalue_yaw))
  ;[1 1 1] Tick (rotation)
  (if (not (`KismetSystemLibrary.IsValid` (`self.ControllerReference`)))
    (bind _asplayer_controller_game_level_thief (cast `/Game/VvVvV_Reloaded/Blueprints/Level_2_GameLevel/PlayerController_GameLevel_Thief` (`self.GetController`)))
    (set `self.ControllerReference` _asplayer_controller_game_level_thief))
  (`self.ServerSetActorRotation` _returnvalue)
  (`self.SetActorRotation` _returnvalue))

(event `ServerSetActorRotation`
  (params (Rotation :type "Rotator Structure"))
  ;[1 1 1] Tick (rotation)
  (`self.SetActorRotation` Rotation)
  (`self.ClientSetActorRotation` Rotation))

(event `ClientSetActorRotation`
  (params (Rotation :type "Rotator Structure"))
  ;[1 1 1] Tick (rotation)
  (`self.SetActorRotation` Rotation))

(event `Key|LeftMouseButton`
  (params (Key :type "Key Structure" :default "AnyKey"))
  (bind (_returnvalue_roll _returnvalue_pitch _returnvalue_yaw) (`KismetMathLibrary.BreakRotator` (`KismetMathLibrary.FindLookAtRotation` (`self.K2_GetActorLocation` self) (`.Location` (`GameplayStatics.BreakHitResult` (`PlayerController.GetHitResultUnderCursorByChannel` (`self.ControllerReference`) "TraceTypeQuery1" true))))))
  (bind _returnvalue (`KismetMathLibrary.MakeRotator` 0.0 0.0 _returnvalue_yaw))
  ;[1 1 1] Launch cube !
  (:`Pressed`
    (if (`self.CanLaunchProjectile`)
      (`self.NetworkSpawProjectile` (`KismetMathLibrary.MakeTransform` (+ (* (`KismetMathLibrary.GetForwardVector` _returnvalue) 50.0) (`self.K2_GetActorLocation` self)) _returnvalue))
      (set `self.CanLaunchProjectile` false)
      (`KismetSystemLibrary.Delay` 2.0)
      (set `self.CanLaunchProjectile` true))))

(event `NetworkSpawProjectile`
  (params (Transform :type "Transform Structure"))
  ;[1 1 1] Launch cube !
  (`|SpawnActorFromClass` "/Game/VvVvV_Reloaded/Blueprints/Level_2_GameLevel/Blueprint_Projectile.Blueprint_Projectile_C" Transform "AdjustIfPossibleButAlwaysSpawn" "OverrideRootScale"))

(fn `UserConstructionScript`
  (bind _asplayer_controller_game_level_thief (cast `/Game/VvVvV_Reloaded/Blueprints/Level_2_GameLevel/PlayerController_GameLevel_Thief` (`self.GetController`)))
  (set `self.ControllerReference` _asplayer_controller_game_level_thief))