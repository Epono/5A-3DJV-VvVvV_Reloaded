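; Trap actor that roots any top-down character other than its owner that walks into it.
; It arms two seconds after spawning; an overlap then plays a trigger sound and reveals the cylinder mesh.
; The victim's max walk speed is cached and zeroed for the trap duration, then restored before the actor destroys itself.
; CanTrigger is never cleared after firing, and the TriggerTrap event is an empty stub.
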(event `self.ReceiveBeginPlay`
  (`KismetSystemLibrary.Delay` 2.0)
  (set `self.CanTrigger` true))

(event `self.ReceiveActorBeginOverlap`
  (params (OtherActor :type "Actor Object Reference"))
  (if (`self.CanTrigger`)
    (bind _astop_down_character (cast `/Game/VvVvV_Reloaded/Blueprints/TopDownCharacter` OtherActor))
    (if (!= _astop_down_character (`self.OwnerCharacter`))
      (set `self.OtherCharacterMovement` (`Character.CharacterMovement` _astop_down_character))
      (`GameplayStatics.PlaySoundAtLocation` "/Game/VvVvV_Reloaded/Audio/TrapTriggeringSound.TrapTriggeringSound" (`SceneComponent.K2_GetComponentLocation` (`self.Cylinder`)))
      (`SceneComponent.SetVisibility` (`self.Cylinder`) true true)
      (set `self.MaxWalkSpeed` (`CharacterMovementComponent.MaxWalkSpeed` (`self.OtherCharacterMovement`)))
      (set `CharacterMovementComponent.MaxWalkSpeed` 0.0 (`self.OtherCharacterMovement`))
      (`KismetSystemLibrary.Delay` (`self.TrapDuration`))
      (set `CharacterMovementComponent.MaxWalkSpeed` (`self.MaxWalkSpeed`) (`self.OtherCharacterMovement`))
      (`self.K2_DestroyActor`))))

(event `TriggerTrap`)

(fn `UserConstructionScript`)