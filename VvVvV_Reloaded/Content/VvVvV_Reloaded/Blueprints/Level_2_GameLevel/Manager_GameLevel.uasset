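; Level 2 game manager that runs a timed coin-collecting match for up to four Thief players.
; On start it plays music, randomly spawns coins at spawn points, assigns player materials and updates each HUD countdown.
; Timeout makes everyone lose, while an empty coin check crowns the top score; both share an ending that later teleports players to stepped placement spots.
; Placement follows player index rather than sorted score, and PlayerMaxCoins doubles as first-place slot.
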(event `TimerPlayerName`
  (for _index (range 4)
    (bind _asplayer_character_game_level_thief (cast `/Game/VvVvV_Reloaded/Blueprints/Level_2_GameLevel/PlayerCharacter_GameLevel_Thief` (`GameplayStatics.GetPlayerCharacter` _index)))
    (`/Game/VvVvV_Reloaded/Blueprints/Level_2_GameLevel/PlayerCharacter_GameLevel_Thief.ChangePlayerMaterial` _asplayer_character_game_level_thief _index)))

(event `self.ReceiveBeginPlay`
  ;[1 1 1] Initialisation (musique et pièces)
  (`GameplayStatics.PlaySound2D` "/Game/VvVvV_Reloaded/Audio/BackgroundMusic.BackgroundMusic" 0.02)
  (`KismetSystemLibrary.K2_SetTimerDelegate` (delegate `EndOfGame`) (`self.GameDuration`))
  (`KismetSystemLibrary.K2_SetTimerDelegate` (delegate `TimerPlayerName`) 1.0)
  (bind _outactors (`GameplayStatics.GetAllActorsOfClass` "/Game/VvVvV_Reloaded/Blueprints/Level_2_GameLevel/Blueprint_CoinSpawnPoint.Blueprint_CoinSpawnPoint_C"))
  (for _array_element _outactors
    (if (`KismetMathLibrary.RandomBool`)
      (`/Game/VvVvV_Reloaded/Blueprints/Level_2_GameLevel/Blueprint_CoinSpawnPoint.SpawnCoin` _array_element)))
  (`KismetSystemLibrary.K2_SetTimerDelegate` (delegate `CheckCoins`) 1.0 true))

(event `EndOfGame`
  ;[1 1 1] Initialisation (musique et pièces)
  ;[1 1 1] Fin de partie
  (set `self.EndOfTime` true)
  (for _index (range 4) :!label _label
    (bind _asplayer_character_game_level_thief (cast `/Game/VvVvV_Reloaded/Blueprints/Level_2_GameLevel/PlayerCharacter_GameLevel_Thief` (`GameplayStatics.GetPlayerCharacter` _index)))
    (if (`self.EndOfTime`)
      (set `/Game/VvVvV_Reloaded/Blueprints/Level_2_GameLevel/PlayerCharacter_GameLevel_Thief.Winner` false _asplayer_character_game_level_thief)
      (set `/Game/VvVvV_Reloaded/Blueprints/Level_2_GameLevel/PlayerCharacter_GameLevel_Thief.GameOver` true _asplayer_character_game_level_thief :!label _label_2)
      (elif (== (`/Game/VvVvV_Reloaded/Blueprints/Level_2_GameLevel/PlayerCharacter_GameLevel_Thief.Score` _asplayer_character_game_level_thief) (`self.PlayerMaxCoins`))
        (set `/Game/VvVvV_Reloaded/Blueprints/Level_2_GameLevel/PlayerCharacter_GameLevel_Thief.Winner` true _asplayer_character_game_level_thief)
        (goto _label_2))))
  (`KismetSystemLibrary.Delay` 5.0)
  (for _index_2 (range 4)
    (bind _asplayer_character_game_level_thief_2 (cast `/Game/VvVvV_Reloaded/Blueprints/Level_2_GameLevel/PlayerCharacter_GameLevel_Thief` (`GameplayStatics.GetPlayerCharacter` _index_2)))
    (for _index_3 (range 201)
      (if (== _index_3 (`/Game/VvVvV_Reloaded/Blueprints/Level_2_GameLevel/PlayerCharacter_GameLevel_Thief.Score` _asplayer_character_game_level_thief_2))
        (if (== (`self.PlayerMaxCoins`) -1)
          (set `self.PlayerMaxCoins` _index_2)
          (set `/Game/VvVvV_Reloaded/Blueprints/Level_2_GameLevel/PlayerCharacter_GameLevel_Thief.CanTeleport` true _asplayer_character_game_level_thief_2)
          (`/Game/VvVvV_Reloaded/Blueprints/Level_2_GameLevel/PlayerCharacter_GameLevel_Thief.Server_TeleportPlayer` _asplayer_character_game_level_thief_2 (7230.0 50.0 2600.0))
          (elif (== (`self.2ndPlayer`) -1)
            (set `self.2ndPlayer` _index_2)
            (set `/Game/VvVvV_Reloaded/Blueprints/Level_2_GameLevel/PlayerCharacter_GameLevel_Thief.CanTeleport` true _asplayer_character_game_level_thief_2)
            (`/Game/VvVvV_Reloaded/Blueprints/Level_2_GameLevel/PlayerCharacter_GameLevel_Thief.Server_TeleportPlayer` _asplayer_character_game_level_thief_2 (7230.0 -150.0 2500.0))
            (elif (== (`self.3rdPlayer`) -1)
              (set `self.3rdPlayer` _index_2)
              (set `/Game/VvVvV_Reloaded/Blueprints/Level_2_GameLevel/PlayerCharacter_GameLevel_Thief.CanTeleport` true _asplayer_character_game_level_thief_2)
              (`/Game/VvVvV_Reloaded/Blueprints/Level_2_GameLevel/PlayerCharacter_GameLevel_Thief.Server_TeleportPlayer` _asplayer_character_game_level_thief_2 (7230.0 -350.0 2400.0))
              (elif (== (`self.4thPlayer`) -1)
                (set `self.4thPlayer` _index_2)
                (set `/Game/VvVvV_Reloaded/Blueprints/Level_2_GameLevel/PlayerCharacter_GameLevel_Thief.CanTeleport` true _asplayer_character_game_level_thief_2)
                (`/Game/VvVvV_Reloaded/Blueprints/Level_2_GameLevel/PlayerCharacter_GameLevel_Thief.Server_TeleportPlayer` _asplayer_character_game_level_thief_2 (7230.0 -550.0 2300.0))))))))))

(event `CheckCoins`
  (bind _outactors (`GameplayStatics.GetAllActorsOfClass` "/Game/VvVvV_Reloaded/Blueprints/Level_2_GameLevel/Blueprint_Coin.Blueprint_Coin_C"))
  (if (== (`KismetArrayLibrary.Array_Length` _outactors) 0)
    (`/Engine/EditorBlueprintResources/StandardMacros.DoOnce` false
      (:`Completed`
        (for _index (range 4)
          (bind _asplayer_character_game_level_thief (cast `/Game/VvVvV_Reloaded/Blueprints/Level_2_GameLevel/PlayerCharacter_GameLevel_Thief` (`GameplayStatics.GetPlayerCharacter` _index)))
          (bind _score (`/Game/VvVvV_Reloaded/Blueprints/Level_2_GameLevel/PlayerCharacter_GameLevel_Thief.Score` _asplayer_character_game_level_thief))
          (if (> _score (`self.PlayerMaxCoins`))
            (set `self.PlayerMaxCoins` _score))
          (set `/Game/VvVvV_Reloaded/Blueprints/Level_2_GameLevel/PlayerCharacter_GameLevel_Thief.GameOver` true _asplayer_character_game_level_thief))
        (goto _label)))))

(event `self.ReceiveTick`
  (params (DeltaSeconds :type "Float (single-precision)"))
  ;[1 1 1] Mise à jour du temps restant
  (if (not (`self.EndOfTime`))
    (set `self.TimeElapsed` (+ (`self.TimeElapsed`) DeltaSeconds))
    (for _index (range 4)
      (bind _asplayer_controller_game_level_thief (cast `/Game/VvVvV_Reloaded/Blueprints/Level_2_GameLevel/PlayerController_GameLevel_Thief` (`GameplayStatics.GetPlayerController` _index)))
      (set `/Game/VvVvV_Reloaded/HUD/HUD_GameLevel_Thief.RemainingTime` (- (`self.GameDuration`) (`self.TimeElapsed`)) (`/Game/VvVvV_Reloaded/Blueprints/Level_2_GameLevel/PlayerController_GameLevel_Thief.HUD_Reference` _asplayer_controller_game_level_thief)))))

(event `PlayerPickedUpCoin`
  (params (Coin :type "/Game/VvVvV_Reloaded/Blueprints/Level_2_GameLevel/Blueprint_Coin Object Reference") (PlayerCharacter :type "/Game/VvVvV_Reloaded/Blueprints/Level_2_GameLevel/PlayerCharacter_GameLevel_Thief Object Reference"))
  ;[1 1 1] Pas utilisé
)

(fn `UserConstructionScript`)